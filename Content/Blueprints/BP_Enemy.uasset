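; BP_Enemy is an enemy ship that gives itself a random color scheme and explodes in matching colors.
; SetColor picks body and wing colors from two fixed palettes, applies them through a dynamic M_Base_Ship material, and scales the actor with a spawn timeline.
; SpawnExplosion passes the stored colors to the PS_Explosion emitter at the ship's location.
; Neither event is called within this Blueprint.
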(event `self.SetColor`
  (bind _returnvalue (select `int` (`self.BodyColorIndex`) :`0` (struct :`R` 0.284432 :`G` 0.973958 :`B` 0.191972 :`A` 1.0) :`1` (struct :`R` 0.205011 :`G` 0.239363 :`B` 0.984375 :`A` 1.0) :`2` (struct :`R` 0.921875 :`G` 0.117936 :`B` 0.009603 :`A` 1.0) :`3` (struct :`R` 1.0 :`A` 1.0) :!type "LinearColor Structure"))
  (bind _returnvalue_2 (select `int` (`self.WingColorIndex`) :`0` (struct :`R` 0.994792 :`G` 0.12207 :`B` 0.741616 :`A` 1.0) :`1` (struct :`R` 0.96875 :`G` 0.851579 :`B` 0.04541 :`A` 1.0) :`2` (struct :`R` 0.198603 :`G` 0.920185 :`B` 0.958333 :`A` 1.0) :`3` (struct :`R` 0.892097 :`G` 0.88491 :`B` 0.9375 :`A` 1.0) :!type "LinearColor Structure"))
  (set `self.BodyColorIndex` (`KismetMathLibrary.RandomIntegerInRange` 0 3))
  (set `self.WingColorIndex` (`KismetMathLibrary.RandomIntegerInRange` 0 3))
  (bind _returnvalue_3 (`KismetMaterialLibrary.CreateDynamicMaterialInstance` "/Game/SpaceshipBattle/Materials/M_Base_Ship.M_Base_Ship"))
  (`MaterialInstanceDynamic.SetVectorParameterValue` _returnvalue_3 "Color1" _returnvalue)
  (set `self.PrimaryColor` _returnvalue)
  (`MaterialInstanceDynamic.SetVectorParameterValue` _returnvalue_3 "Color2" _returnvalue_2)
  (`PrimitiveComponent.SetMaterial` (`self.ShipSM`) 0 _returnvalue_3)
  (set `self.SecondryColor` _returnvalue_2)
  (bind (_direction _scale) (`Timeline|SpawnScaleTimeline`)
    (:`Update`
      (`self.SetActorScale3D` (`KismetMathLibrary.Conv_DoubleToVector` _scale)))))

(event `self.SpawnExplosion`
  (bind _returnvalue (`GameplayStatics.SpawnEmitterAtLocation` "/Game/ParticleSystem/PS_Explosion.PS_Explosion" (`self.K2_GetActorLocation`)))
  (`ParticleSystemComponent.SetColorParameter` _returnvalue "PrimaryColor" (`self.PrimaryColor`))
  (`ParticleSystemComponent.SetColorParameter` _returnvalue "SecondryColor" (`self.SecondryColor`)))

(fn `UserConstructionScript`)